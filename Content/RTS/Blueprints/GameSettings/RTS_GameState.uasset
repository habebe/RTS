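; RTS game state that runs the in-game clock through an RTS_GameTime object, created in the construction script with a default timescale and the current date.
; BeginPlay caches the first player controller, and each Tick advances the clock and pushes the current time to that controller's HUD game-time widget.
; Timescale get and set and current date queries forward to the time object, while SetGameTime is a stub returning false.
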(event EventBeginPlay
  (Utilities|Initialize))

(event EventTick
  (params (DeltaSeconds :type Float%20%28single-precision%29))
  (Utilities|UpdateGameTime DeltaSeconds))

(event EventSetTimescale
  (params (Timescale :type Float%20%28single-precision%29))
  ;[1 1 1] Event: GameTime
  (Class|RTSGameTime|SetTimescale (Variables|Default|GetGameTime) Timescale))

(fn ConstructionScript
  (Utilities|InitializeGameTimeObject))

(fn GetTimescale
  (return (Class|RTSGameTime|GetTimeScale (Variables|Default|GetGameTime))))

(fn GetCurrentDateTime
  (return (Class|RTSGameTime|GetCurrent (Variables|Default|GetGameTime))))

(fn SetGameTime
  (params (DateTime :type Date%20Time%20Structure))
  (return false))