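; RTS sun actor that drives the level's sun from the game's simulated calendar time.
; On begin play it caches the RTS game state, stores the current time scale and subscribes to time scale changes.
; Every tick it copies the game state's current date and time into its SunPosition and calls UpdateSun.
; The stored time scale is not otherwise used in this graph.
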(event Custom|GetTimescale
  (params (Time%20Scale :type Float%20%28single-precision%29))
  ;[1 1 1] Custom Event
  (Variables|Default|SetTimescale Time%20Scale))

(event EventBeginPlay
  (bind _output_get (Variables|Default|SetGameState (.AsRTS%20Game%20State (Utilities|Casting|CastToRTS_GameState (Game|GetGameState)))))
  (EventDispatchers|BindEventtoTimeScaleControl _output_get (EventDispatchers|CreateEvent :!event Custom|GetTimescale))
  (bind _timescale (Default|GetTimescale (Variables|Default|GetGameState)))
  (Variables|Default|SetTimescale _timescale))

(event EventTick
  (params (DeltaSeconds :type Float%20%28single-precision%29))
  (bind _sunposition (Variables|RTS|References|GetSunPosition))
  (bind _current_date_time (Default|GetCurrentDateTime (Variables|Default|GetGameState)))
  (Variables|/SunPosition/BP_SunPosition.BP_SunPosition_C|SetYear _sunposition (.year _current_date_time))
  (Variables|/SunPosition/BP_SunPosition.BP_SunPosition_C|SetMonth _sunposition (.month _current_date_time))
  (Variables|/SunPosition/BP_SunPosition.BP_SunPosition_C|SetDay _sunposition (.day _current_date_time))
  (Variables|/SunPosition/BP_SunPosition.BP_SunPosition_C|SetHours _sunposition (.hour _current_date_time))
  (Variables|/SunPosition/BP_SunPosition.BP_SunPosition_C|SetMinutes _sunposition (.minute _current_date_time))
  (Variables|/SunPosition/BP_SunPosition.BP_SunPosition_C|SetSeconds _sunposition (.second _current_date_time))
  (Default|UpdateSun _sunposition))

(fn ConstructionScript)