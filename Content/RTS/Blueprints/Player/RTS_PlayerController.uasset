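; RTS player controller that drives the RTS_CameraPawn with move, pan and zoom input and shows the game-time HUD.
; CameraSettings configures speeds, limits and debug printing, and its MovementHandler selects Blueprint, floating-pawn or RTS_CameraActionHandler implementations for actions.
; The handler, constructed at BeginPlay, also tracks action state through Begin, End and Is checks.
; An edge-scroll X macro exists but is not called here, and PanReset input always uses the Blueprint path.
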(event EventBeginPlay
  (Utilities|Initialize)
  (Utilities|SpawnWidget)
  (UserInterface|Viewport|AddtoViewport (Variables|Default|GetHUDGametimeWidget) 0)
  (CallFunction|SetHUDVisibility "Visible"))

(event EventUpdateCameraSettings
  (params (CameraSettings :type RTS%20Camera%20Settings%20Structure) (InitializePosition :type Boolean))
  ;[1 1 1] Event: UpdateCameraSettings
  (CallFunction|SetCameraSettings CameraSettings InitializePosition))

(event Input|ActionEvents|InputActionZoomReset
  (params (Key :type Key%20Structure :default "None"))
  ;[1 1 1] Event:Zoom
  (:Pressed
    (Utilities|ActionZoomReset)))

(event Input|ActionEvents|InputActionZoomIn
  (params (Key :type Key%20Structure :default "None"))
  ;[1 1 1] Event:Zoom
  (:Pressed
    (Utilities|ActionZoom 1.0)))

(event Input|ActionEvents|InputActionZoomOut
  (params (Key :type Key%20Structure :default "None"))
  ;[1 1 1] Event:Zoom
  (:Pressed
    (Utilities|ActionZoom -1.0)))

(event Input|ActionEvents|InputActionPan
  (params (Key :type Key%20Structure :default "None"))
  (:Pressed
    (Utilities|BeginAction "Pan" 0.0))
  (:Released
    (Utilities|EndAction "Pan")))

(event Input|ActionEvents|InputActionPanReset
  (params (Key :type Key%20Structure :default "None"))
  (:Pressed
    (Utilities|ActionPanResetUsingBlueprint (Variables|Default|GetCameraReference) (.cameraangle (Variables|Default|GetCameraSettings)))))

(event Input|AxisEvents|InputAxisMoveForward
  (params (AxisValue :type Float%20%28single-precision%29))
  ;[1 1 1] Event: Movement
  (Utilities|ActionMove AxisValue (stale Input|AxisEvents|InputAxisMoveRight AxisValue)))

(event Input|AxisEvents|InputAxisMoveRight
  (params (AxisValue :type Float%20%28single-precision%29))
  ;[1 1 1] Event: Movement
  (Utilities|ActionMove (stale Input|AxisEvents|InputAxisMoveForward AxisValue) AxisValue) ; enters at Right
)

(event Input|MouseEvents|MouseX
  (params (AxisValue :type Float%20%28single-precision%29))
  (bind _camerasettings (Variables|Default|GetCameraSettings))
  (Utilities|IsAction "Pan"
    (:True
      (Utilities|ActionPan AxisValue (stale Input|MouseEvents|MouseY AxisValue) (Variables|Default|GetCameraReference) (.panspeed _camerasettings) (.minimumpanpitch _camerasettings) (.maximumpanpitch _camerasettings)))))

(event Input|MouseEvents|MouseY
  (params (AxisValue :type Float%20%28single-precision%29))
  (bind _camerasettings (Variables|Default|GetCameraSettings))
  (Utilities|IsAction "Pan"
    (:True
      (Utilities|ActionPan (stale Input|MouseEvents|MouseX AxisValue) AxisValue (Variables|Default|GetCameraReference) (.panspeed _camerasettings) (.minimumpanpitch _camerasettings) (.maximumpanpitch _camerasettings)))))

(fn ConstructionScript)

(fn SetCameraSettings
  (params (CameraSettings :type RTS%20Camera%20Settings%20Structure) (InitializePosition :type Boolean))
  (Variables|Default|SetCameraSettings CameraSettings)
  (CallFunction|InitializeCamera InitializePosition)
  (return))

(fn InitializeCamera
  (params (InitializePosition :type Boolean))
  (bind _camerasettings (Variables|Default|GetCameraSettings))
  (bind _camerareference (Variables|Default|GetCameraReference))
  (if (Utilities|IsValid _camerareference)
    (Rendering|SetVisibility (Variables|/Game/RTS/Blueprints/Player/RTS_CameraPawn.RTS_CameraPawn_C|GetSphere _camerareference) (.showsphere _camerasettings) true)
    (if InitializePosition
      (Variables|/Script/Engine.SpringArmComponent|SetTargetArmLength (Variables|/Game/RTS/Blueprints/Player/RTS_CameraPawn.RTS_CameraPawn_C|GetSpringArm _camerareference) (.cameradistance _camerasettings))
      (Transformation|SetActorRotation _camerareference (.cameraangle _camerasettings)))))

(fn SetHUDVisibility
  (params (GametimeHUD :type ESlateVisibility%20Enum :default "Visible"))
  (Widget|SetVisibility (Variables|Default|GetHUDGametimeWidget) GametimeHUD))