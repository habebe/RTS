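; RTS startup task container that holds the set of tasks for RTS startup.
; Initialize constructs an instance of each class in TaskTypes, with the container as outer, and stores it in the Tasks array.
; GetNumberOfTasks and GetTask expose the created tasks by count and index.
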(fn Initialize
  (params (Object :type RTS%20Startup%20Widget%20Object%20Reference))
  (for _array_element (Variables|Default|GetTaskTypes)
    (bind _returnvalue (Game|ConstructObjectfromClass _array_element self))
    (bind _output_get (LocalVariables|SetTask _returnvalue))
    (Utilities|Array|Add (Variables|Default|GetTasks) _output_get)))

(fn GetNumberOfTasks
  (return (Utilities|Array|Length (Variables|Default|GetTasks))))

(fn GetTask
  (params (Index :type Integer))
  (return (Utilities|Array|Get(acopy) (Variables|Default|GetTasks) Index)))