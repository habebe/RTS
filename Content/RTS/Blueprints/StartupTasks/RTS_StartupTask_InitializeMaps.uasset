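; RTS startup task named for map initialization, run by a startup controller, though its graph contains no map-loading logic.
; PerformTask stores the controller and simulates three steps, each a timed delay followed by a progress increment.
; It then reports full progress to the controller and marks itself completed, provided the controller casts to RTS_StartupWidget.
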(event EventPerformTask
  (params (Controller :type RTS%20Startup%20Controller%20IF%20Interface))
  (Variables|Default|SetController Controller)
  (Variables|Default|SetCurrentIndex 0)
  (Variables|Default|SetTotalSize 3)
  (Utilities|FlowControl|Delay self (Variables|Default|GetDelayValue))
  (CallFunction|IncrementTaskProgress 1)
  (Utilities|FlowControl|Delay self (Variables|Default|GetDelayValue))
  (CallFunction|IncrementTaskProgress 1)
  (Utilities|FlowControl|Delay self (Variables|Default|GetDelayValue))
  (CallFunction|IncrementTaskProgress 1)
  (Default|SetTaskProgress (Variables|Default|GetController) self 1.0)
  (bind _asrts_startup_widget (Utilities|Casting|CastToRTS_StartupWidget (Variables|Default|GetController)))
  (CallFunction|SetTaskCompleted _asrts_startup_widget))