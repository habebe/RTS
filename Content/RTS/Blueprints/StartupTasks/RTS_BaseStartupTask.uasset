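; Base startup task for the RTS game, run by a controller and tracking its own status, name, progress and error message.
; Initialization sets the status text and binds to the controller's run dispatcher, whose event calls PerformTask to do the work.
; Completion updates status, notifies the controller and unbinds, while failure only records status and message.
; Helpers report fractional progress to the controller and wrap a delay.
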(event EventRunTask
  (params (Controller :type RTS%20Startup%20Controller%20IF%20Interface))
  (CallFunction|PerformTask Controller))

(event EventInitializeTask
  (params (Controller :type RTS%20Startup%20Widget%20Object%20Reference))
  (Variables|Default|SetStatus "NewEnumerator3")
  (Default|SetStatusText Controller self (Variables|Default|GetName))
  (EventDispatchers|BindEventtoRunEventDispatcher Controller (delegate EventRunTask)))

(event EventUnitializeTask
  (params (Controller :type RTS%20Startup%20Widget%20Object%20Reference))
  (Default|SetTaskCompleted Controller self)
  (EventDispatchers|UnbindEventfromRunEventDispatcher Controller (delegate EventRunTask)))

(fn SetTaskCompleted
  (params (Controller :type RTS%20Startup%20Widget%20Object%20Reference))
  (Variables|Default|SetStatus "NewEnumerator1")
  (CallFunction|UnitializeTask Controller))

(fn SetTaskFailed
  (params (ErrorMessage :type Text))
  (Utilities|FlowControl|Sequence
    (:then_0
      (Variables|Default|SetStatus "NewEnumerator2"))
    (:then_1
      (Variables|Default|SetErrorMessage ErrorMessage))))

(fn IncrementTaskProgress
  (params (incrementValue :type Integer))
  (Default|SetTaskProgress (Variables|Default|GetController) self (Math|Float|SafeDivide (Math|Conversions|ToFloat(Integer) (+ (Variables|Default|GetCurrentIndex) 1)) (Math|Conversions|ToFloat(Integer) (Variables|Default|GetTotalSize))))
  (Variables|Default|SetCurrentIndex (+ (Variables|Default|GetCurrentIndex) incrementValue)))

(fn GetErrorMessage
  (return (Variables|Default|GetErrorMessage)))

(fn GetName
  (return (Variables|Default|GetName)))

(fn GetStatus
  (return (Variables|Default|GetStatus)))